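; BP_DoorMaster is an interactable door that moves the third-person player to a linked exit point.
; Overlapping its box shows a prompt widget, enables input and opens a gate that lets the interact action fire; leaving reverses this.
; Interacting locks player input, cubic-blends the camera to a view target, teleports the character to the exit's TPPoint, then blends back and restores input.
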(event OnComponentBeginOverlap(Box)
  (params (OverlappedComponent :type Primitive%20Component%20Object%20Reference) (OtherActor :type Actor%20Object%20Reference) (OtherComp :type Primitive%20Component%20Object%20Reference) (OtherBodyIndex :type Integer) (bFromSweep :type Boolean) (SweepResult :type Hit%20Result%20Structure%20%28by%20ref%29))
  (bind _returnvalue (Game|GetPlayerController 0))
  (bind _returnvalue_2 (Game|GetPlayerCharacter 0))
  (bind _returnvalue_3 (Game|GetPlayerController 0))
  (Rendering|SetVisibility (Variables|Default|GetWidget) true false)
  (bind _asbp_third_person_character (Utilities|Casting|CastToBP_ThirdPersonCharacter OtherActor))
  (Input|EnableInput (Game|GetPlayerController 0))
  (Utilities|FlowControl|Gate true) ; enters at Open
)

(event OnComponentEndOverlap(Box)
  (params (OverlappedComponent :type Primitive%20Component%20Object%20Reference) (OtherActor :type Actor%20Object%20Reference) (OtherComp :type Primitive%20Component%20Object%20Reference) (OtherBodyIndex :type Integer))
  (bind _returnvalue (Game|GetPlayerController 0))
  (bind _returnvalue_2 (Game|GetPlayerCharacter 0))
  (bind _returnvalue_3 (Game|GetPlayerController 0))
  (Rendering|SetVisibility (Variables|Default|GetWidget) false false)
  (Utilities|Casting|CastToBP_ThirdPersonCharacter OtherActor)
  (Input|DisableInput (Game|GetPlayerController 0))
  (Utilities|FlowControl|Gate true) ; enters at Close
)

(event Input|EnhancedActionEvents|EnhancedInputActionIA_Interact
  (params (ActionValue :type Boolean) (ElapsedSeconds :type Float%20%28double-precision%29) (TriggeredSeconds :type Float%20%28double-precision%29) (InputAction :type Input%20Action%20Object%20Reference :default "/Game/ThirdPerson/Input/Actions/IA_Interact.IA_Interact"))
  (bind _returnvalue (Game|GetPlayerController 0))
  (bind _returnvalue_2 (Game|GetPlayerCharacter 0))
  (bind _returnvalue_3 (Game|GetPlayerController 0))
  (:Completed
    (Utilities|FlowControl|Gate true
      (:Exit
        (Input|DisableInput (Game|GetPlayerCharacter 0) _returnvalue)
        (Game|Player|SetViewTargetwithBlend _returnvalue (Variables|Default|GetNew%20View%20Target) (Variables|Default|GetBlend%20Time) "VTBlend_Cubic" 0.0 false)
        (Utilities|FlowControl|Delay (+ (Variables|Default|GetBlend%20Time) 0.2))
        (Transformation|SetActorLocation (stale OnComponentBeginOverlap(Box) _asbp_third_person_character) (+ (Transformation|GetWorldLocation (Variables|/Game/Ewan/BP_Checkpoint.BP_Checkpoint_C|GetTPPoint (Variables|Default|GetExitPoint))) "") false true)
        (Game|Player|SetViewTargetwithBlend _returnvalue_3 _returnvalue_2 0.2 "VTBlend_Cubic" 0.0 false)
        (Utilities|FlowControl|Delay 0.2)
        (Input|EnableInput _returnvalue_2 _returnvalue_3)))))

(event EventBeginPlay
  (|CallParentFunction) ; This node is disabled and will not be called.\nDrag off pins to build functionality.
)

(event Collision|EventActorBeginOverlap
  (params (OtherActor :type Actor%20Object%20Reference))
  (|CallParentFunction OtherActor) ; This node is disabled and will not be called.\nDrag off pins to build functionality.
)

(event EventTick
  (params (DeltaSeconds :type Float%20%28single-precision%29))
  (|CallParentFunction DeltaSeconds) ; This node is disabled and will not be called.\nDrag off pins to build functionality.
)

(fn ConstructionScript
  (|CallParentFunction))