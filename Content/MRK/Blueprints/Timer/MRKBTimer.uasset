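; MRKBTimer is a countdown timer that can pause itself and freeze enemies.
; On BeginPlay it creates the MRKWTimer widget, caches all BP_Enemy_Base actors and unfreezes.
; Each Tick subtracts delta time from the widget's clamped value unless frozen.
; Freeze and unfreeze toggle the cached enemies' CustomTimeDilation, while save and load are delegated to the widget, which holds the time value.
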(event EventTick
  (params (DeltaSeconds :type Float%20%28single-precision%29))
  (Variables|Default|SetVDelta DeltaSeconds)
  (CallFunction|FUpdate))

(event EventBeginPlay
  (CallFunction|FInitialize))

(fn ConstructionScript)

(fn FInitialize
  (CallFunction|FInitializeWidget)
  (CallFunction|FInitializeEnemies)
  (CallFunction|FUnfreeze))

(fn FInitializeWidget
  (bind _returnvalue (UserInterface|CreateWidget "/Game/MRK/Blueprints/Timer/MRKWTimer.MRKWTimer_C"))
  (bind _output_get (Variables|Default|SetVWidget _returnvalue))
  (UserInterface|Viewport|AddtoViewport _output_get 0))

(fn FInitializeEnemies
  (bind _outactors (Actor|GetAllActorsOfClass "/Game/Enemy/BP_Enemy_Base.BP_Enemy_Base_C"))
  (Variables|Default|SetVEnemies _outactors))

(fn FUpdate
  (CallFunction|FUpdateWidget))

(fn FUpdateWidget
  (if (not (Variables|Default|GetVFreezed))
    (Variables|/Game/MRK/Blueprints/Timer/MRKWTimer.MRKWTimer_C|SetVValue (Variables|Default|GetVWidget) (Math|Float|Clamp(Float) (- (Variables|/Game/MRK/Blueprints/Timer/MRKWTimer.MRKWTimer_C|GetVValue (Variables|Default|GetVWidget)) (Variables|Default|GetVDelta)) 0.0 6e+02))))

(fn FFreeze
  (Variables|Default|SetVFreezed true)
  (for _array_element (Variables|Default|GetVEnemies)
    (Variables|/Script/Engine.Actor|SetCustomTimeDilation _array_element 0.0)))

(fn FUnfreeze
  (Variables|Default|SetVFreezed false)
  (for _array_element (Variables|Default|GetVEnemies)
    (Variables|/Script/Engine.Actor|SetCustomTimeDilation _array_element 1.0)))

(fn FSave
  (Default|FSave (Variables|Default|GetVWidget)))

(fn FLoad
  (Default|FLoad (Variables|Default|GetVWidget)))