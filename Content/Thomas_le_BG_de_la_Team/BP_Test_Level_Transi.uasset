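; BP_Test_Level_Transi is a level transition trigger that moves the game to the level named by LevelName.
; Any overlap on its Trigger shows the WBP_Transi_Level_1 fade-in widget, waits briefly, saves through BP_Timer, then opens the level.
; FLoad on BP_Timer and the GameInstance's background music call follow OpenLevel in the same chain, so they are issued from the outgoing world.
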(event OnComponentBeginOverlap(Trigger)
  (params (OverlappedComponent :type Primitive%20Component%20Object%20Reference) (OtherActor :type Actor%20Object%20Reference) (OtherComp :type Primitive%20Component%20Object%20Reference) (OtherBodyIndex :type Integer) (bFromSweep :type Boolean) (SweepResult :type Hit%20Result%20Structure%20%28by%20ref%29))
  (bind _returnvalue (UserInterface|CreateWidget "/Game/Widgets/Transi_Level/WBP_Transi_Level_1.WBP_Transi_Level_1_C"))
  (UserInterface|Viewport|AddtoViewport _returnvalue 0)
  (Default|FadeinTransi _returnvalue)
  (Utilities|FlowControl|Delay 3.0)
  (bind _returnvalue_2 (Actor|GetActorOfClass "/Game/Widgets/Timer/BP_Timer.BP_Timer_C"))
  (Default|FSave _returnvalue_2)
  (Game|OpenLevel(byName) (Variables|Default|GetLevel%20Name))
  (bind _returnvalue_3 (Actor|GetActorOfClass "/Game/Widgets/Timer/BP_Timer.BP_Timer_C"))
  (Default|FLoad _returnvalue_3)
  (bind _asbp_game_instance (Utilities|Casting|CastToBP_GameInstance (Game|GetGameInstance)))
  (Default|PlayMusic _asbp_game_instance "/Game/Thomas_le_BG_de_la_Team/Music_BP/Music/SC_Background_Music.SC_Background_Music" 0.5))

(fn ConstructionScript)