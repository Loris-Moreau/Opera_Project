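; BP_Camera_Start is a level intro camera that briefly holds the view before handing it to the player.
; On BeginPlay it shows the WBP_Transi_Level widget with a fade-out transition, disables player character input and switches the view target to itself.
; After a fixed delay it starts a cubic blend to the player character and re-enables input immediately, without waiting for the blend to finish.
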(event EventBeginPlay
  (bind _returnvalue (Game|GetPlayerController 0))
  (bind _returnvalue_2 (Game|GetPlayerCharacter 0))
  (bind _returnvalue_3 (UserInterface|CreateWidget "/Game/Thomas_le_BG_de_la_Team/Transi_Level/WBP_Transi_Level.WBP_Transi_Level_C"))
  (UserInterface|Viewport|AddtoViewport _returnvalue_3 0)
  (Default|FadeOutTransi _returnvalue_3)
  (Input|DisableInput _returnvalue_2 _returnvalue)
  (Game|Player|SetViewTargetwithBlend _returnvalue self 0.0 "VTBlend_PreBlended" 0.0 false)
  (Utilities|FlowControl|Delay 5.5)
  (Game|Player|SetViewTargetwithBlend _returnvalue _returnvalue_2 3.0 "VTBlend_Cubic" 0.0 false)
  (Input|EnableInput _returnvalue_2 _returnvalue))

(fn ConstructionScript)