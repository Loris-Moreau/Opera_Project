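; BP_FinalDoor is the final door, showing a prompt widget and accepting the interact input while the player is in its trigger box.
; On player overlap it polls CanEnterDoor every second, then enables input and opens a Gate, which closes on leaving.
; Interacting disables player input, freezes the first found enemy AI controller, waits through a placeholder animation delay, deletes the Leaderboard save and sets that AI passive.
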(event OnComponentBeginOverlap(TriggerBox)
  (params (OverlappedComponent :type Primitive%20Component%20Object%20Reference) (OtherActor :type Actor%20Object%20Reference) (OtherComp :type Primitive%20Component%20Object%20Reference) (OtherBodyIndex :type Integer) (bFromSweep :type Boolean) (SweepResult :type Hit%20Result%20Structure%20%28by%20ref%29))
  (bind _widget (Variables|Default|GetWidget))
  (Utilities|FlowControl|Sequence
    (:then_0
      (if (Game|IsGamePaused)
        (Rendering|SetVisibility _widget false false)
        (else
          (if (== (Utilities|GetClass OtherActor) "/Game/ThirdPerson/Blueprints/BP_ThirdPersonCharacter.BP_ThirdPersonCharacter_C") :!label _label
            (Rendering|SetVisibility _widget true false)
            (bind _asbp_third_person_character (Utilities|Casting|CastToBP_ThirdPersonCharacter OtherActor))
            (if (Variables|/Game/ThirdPerson/Blueprints/BP_ThirdPersonCharacter.BP_ThirdPersonCharacter_C|GetCanEnterDoor _asbp_third_person_character) :!label _label_2
              (Input|EnableInput (Game|GetPlayerController 0))
              (Utilities|FlowControl|Gate true) ; enters at Open
              (else
                (Utilities|FlowControl|Delay 1.0)
                (goto _label_2)))))))
    (:then_1
      (bind _returnvalue (Actor|GetActorOfClass "/Game/ThirdPerson/Blueprints/BP_ThirdPersonCharacter.BP_ThirdPersonCharacter_C"))
      (if (Variables|/Game/ThirdPerson/Blueprints/BP_ThirdPersonCharacter.BP_ThirdPersonCharacter_C|GetisDead? _returnvalue)
        (Rendering|SetVisibility _widget false false)
        (else
          (goto _label))))
    (:then_2
      (goto _label))))

(event OnComponentEndOverlap(TriggerBox)
  (params (OverlappedComponent :type Primitive%20Component%20Object%20Reference) (OtherActor :type Actor%20Object%20Reference) (OtherComp :type Primitive%20Component%20Object%20Reference) (OtherBodyIndex :type Integer))
  (Rendering|SetVisibility (Variables|Default|GetWidget) false false)
  (Utilities|Casting|CastToBP_ThirdPersonCharacter OtherActor)
  (Input|DisableInput (Game|GetPlayerController 0))
  (Utilities|FlowControl|Gate true) ; enters at Close
)

(event Input|EnhancedActionEvents|EnhancedInputActionIA_Interact
  (params (ActionValue :type Boolean) (ElapsedSeconds :type Float%20%28double-precision%29) (TriggeredSeconds :type Float%20%28double-precision%29) (InputAction :type Input%20Action%20Object%20Reference :default "/Game/ThirdPerson/Input/Actions/Default/IA_Interact.IA_Interact"))
  (:Completed
    (Utilities|FlowControl|Gate true
      (:Exit
        (Rendering|SetVisibility (Variables|Default|GetWidget) false false)
        (Input|DisableInput (Game|GetPlayerCharacter 0) (Game|GetPlayerController 0))
        (Variables|/Script/Engine.SpringArmComponent|SetbEnableCameraLag (Variables|/Game/ThirdPerson/Blueprints/BP_ThirdPersonCharacter.BP_ThirdPersonCharacter_C|GetSpringArm (stale OnComponentBeginOverlap(TriggerBox) _asbp_third_person_character)) false)
        (Variables|/Game/ThirdPerson/Blueprints/BP_ThirdPersonCharacter.BP_ThirdPersonCharacter_C|SetCanEnterDoor (stale OnComponentBeginOverlap(TriggerBox) _asbp_third_person_character) false)
        (bind _outactors (Actor|GetAllActorsOfClass "/Game/Enemy/BP_Enemy_Base.BP_Enemy_Base_C"))
        (if (> (Utilities|Array|Length _outactors) 0)
          ;[1 1 1] Freeze Enemy
          (bind _returnvalue (Actor|GetActorOfClass "/Game/Enemy/Behaviour/AIC_Enemy_Base.AIC_Enemy_Base_C"))
          (Default|SetStateFrozen _returnvalue))
        ;[1 1 1] To be replaced by final animation
        (Utilities|FlowControl|Delay 2e+01)
        (SaveGame|DeleteGameinSlot "Leaderboard")
        (if (> (Utilities|Array|Length _outactors) 0)
          (Default|SetStatePassive _returnvalue))))))

(event EventBeginPlay
  (|CallParentFunction) ; This node is disabled and will not be called.\nDrag off pins to build functionality.
)

(event Collision|EventActorBeginOverlap
  (params (OtherActor :type Actor%20Object%20Reference))
  (|CallParentFunction OtherActor) ; This node is disabled and will not be called.\nDrag off pins to build functionality.
)

(event EventTick
  (params (DeltaSeconds :type Float%20%28single-precision%29))
  (|CallParentFunction DeltaSeconds) ; This node is disabled and will not be called.\nDrag off pins to build functionality.
)

(fn ConstructionScript
  (|CallParentFunction))