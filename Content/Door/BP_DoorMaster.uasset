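; Base door actor that teleports the player to a linked exit point behind a camera blend.
; Trigger overlap shows a prompt and, once the player can enter, opens a gate for the Interact input.
; Interacting locks input and camera lag, blends to a target view, teleports, then restores both.
; An enemy AI controller is frozen meanwhile, then set to investigate; an older spring-arm blend remains unused.
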(event OnComponentBeginOverlap(TriggerBox)
  (params (OverlappedComponent :type Primitive%20Component%20Object%20Reference) (OtherActor :type Actor%20Object%20Reference) (OtherComp :type Primitive%20Component%20Object%20Reference) (OtherBodyIndex :type Integer) (bFromSweep :type Boolean) (SweepResult :type Hit%20Result%20Structure%20%28by%20ref%29))
  (bind _returnvalue (Game|GetPlayerCharacter 0))
  (bind _returnvalue_2 (Game|GetPlayerController 0))
  (bind _widget (Variables|Default|GetWidget))
  (bind _returnvalue_3 (Transformation|GetActorLocation _returnvalue_2))
  (Utilities|FlowControl|Sequence
    (:then_0
      (if (Game|IsGamePaused)
        (Rendering|SetVisibility _widget false false)
        (else
          (if (== (Utilities|GetClass OtherActor) "/Game/ThirdPerson/Blueprints/BP_ThirdPersonCharacter.BP_ThirdPersonCharacter_C") :!label _label
            (Rendering|SetVisibility _widget true false)
            (bind _asbp_third_person_character (Utilities|Casting|CastToBP_ThirdPersonCharacter OtherActor))
            (if (Variables|/Game/ThirdPerson/Blueprints/BP_ThirdPersonCharacter.BP_ThirdPersonCharacter_C|GetCanEnterDoor _asbp_third_person_character) :!label _label_2
              (Input|EnableInput (Game|GetPlayerController 0))
              (Utilities|FlowControl|Gate true) ; enters at Open
              (else
                (Utilities|FlowControl|Delay 1.0)
                (goto _label_2)))))))
    (:then_1
      (bind _returnvalue_4 (Actor|GetActorOfClass "/Game/ThirdPerson/Blueprints/BP_ThirdPersonCharacter.BP_ThirdPersonCharacter_C"))
      (if (Variables|/Game/ThirdPerson/Blueprints/BP_ThirdPersonCharacter.BP_ThirdPersonCharacter_C|GetisDead? _returnvalue_4)
        (Rendering|SetVisibility _widget false false)
        (else
          (goto _label))))
    (:then_2
      (goto _label))))

(event OnComponentEndOverlap(TriggerBox)
  (params (OverlappedComponent :type Primitive%20Component%20Object%20Reference) (OtherActor :type Actor%20Object%20Reference) (OtherComp :type Primitive%20Component%20Object%20Reference) (OtherBodyIndex :type Integer))
  (bind _returnvalue (Game|GetPlayerCharacter 0))
  (bind _returnvalue_2 (Game|GetPlayerController 0))
  (bind _returnvalue_3 (Transformation|GetActorLocation _returnvalue_2))
  (Rendering|SetVisibility (Variables|Default|GetWidget) false false)
  (Utilities|Casting|CastToBP_ThirdPersonCharacter OtherActor)
  (Input|DisableInput (Game|GetPlayerController 0))
  (Utilities|FlowControl|Gate true) ; enters at Close
)

(event Input|EnhancedActionEvents|EnhancedInputActionIA_Interact
  (params (ActionValue :type Boolean) (ElapsedSeconds :type Float%20%28double-precision%29) (TriggeredSeconds :type Float%20%28double-precision%29) (InputAction :type Input%20Action%20Object%20Reference :default "/Game/ThirdPerson/Input/Actions/Default/IA_Interact.IA_Interact"))
  (bind _returnvalue (Game|GetPlayerCharacter 0))
  (bind _returnvalue_2 (Game|GetPlayerController 0))
  (bind _returnvalue_3 (Transformation|GetActorLocation _returnvalue_2))
  (:Completed
    (Utilities|FlowControl|Gate true
      (:Exit
        (Rendering|SetVisibility (Variables|Default|GetWidget) false false)
        (Input|DisableInput (Game|GetPlayerCharacter 0) (Game|GetPlayerController 0))
        (Variables|/Script/Engine.SpringArmComponent|SetbEnableCameraLag (Variables|/Game/ThirdPerson/Blueprints/BP_ThirdPersonCharacter.BP_ThirdPersonCharacter_C|GetSpringArm (stale OnComponentBeginOverlap(TriggerBox) _asbp_third_person_character)) false)
        (Variables|/Game/ThirdPerson/Blueprints/BP_ThirdPersonCharacter.BP_ThirdPersonCharacter_C|SetCanEnterDoor (stale OnComponentBeginOverlap(TriggerBox) _asbp_third_person_character) false)
        (bind _outactors (Actor|GetAllActorsOfClass "/Game/Enemy/BP_Enemy_Base.BP_Enemy_Base_C"))
        (if (> (Utilities|Array|Length _outactors) 0)
          ;[1 1 1] Freeze Enemy
          (bind _returnvalue_4 (Actor|GetActorOfClass "/Game/Enemy/Behaviour/AIC_Enemy_Base.AIC_Enemy_Base_C"))
          (Default|SetStateFrozen _returnvalue_4))
        (Game|Player|SetViewTargetwithBlend (Game|GetPlayerController 0) (Variables|Default|GetNew%20View%20Target) (Variables|Default|GetBlend%20Time) "VTBlend_EaseInOut" 5.0 false)
        (Utilities|FlowControl|Delay (+ (Variables|Default|GetBlend%20Time) 0.2))
        (bind _asbp_third_person_character (Utilities|Casting|CastToBP_ThirdPersonCharacter _returnvalue))
        (Transformation|SetActorLocation _asbp_third_person_character (+ (Transformation|GetWorldLocation (Variables|/Game/ThirdPerson/BP_Checkpoint.BP_Checkpoint_C|GetTPPoint (Variables|Default|GetExitPoint))) "") false true)
        (Utilities|FlowControl|Delay 0.5)
        (Game|Player|SetViewTargetwithBlend _returnvalue_2 _returnvalue 0.2 "VTBlend_EaseInOut" 5.0 false)
        (Utilities|FlowControl|Delay 0.2)
        (Variables|/Script/Engine.SpringArmComponent|SetbEnableCameraLag (Variables|/Game/ThirdPerson/Blueprints/BP_ThirdPersonCharacter.BP_ThirdPersonCharacter_C|GetSpringArm _asbp_third_person_character) true)
        (Variables|/Game/ThirdPerson/Blueprints/BP_ThirdPersonCharacter.BP_ThirdPersonCharacter_C|SetCanEnterDoor _asbp_third_person_character true)
        (Input|EnableInput _returnvalue _returnvalue_2)
        (if (> (Utilities|Array|Length _outactors) 0)
          ;[1 1 1] UnFreeze Enemy
          (bind _returnvalue_5 (Actor|GetActorOfClass "/Game/Enemy/Behaviour/AIC_Enemy_Base.AIC_Enemy_Base_C"))
          (bind _returnvalue_6 (Actor|GetActorOfClass "/Game/Enemy/BP_Enemy_Base.BP_Enemy_Base_C"))
          (Default|SetStateInvestigating _returnvalue_5 (Math|Vector|MakeVector (.x _returnvalue_3) (.y _returnvalue_3) (.z (Transformation|GetActorLocation _returnvalue_6)))))))))

(event EventBeginPlay
  (|CallParentFunction) ; This node is disabled and will not be called.\nDrag off pins to build functionality.
)

(event Collision|EventActorBeginOverlap
  (params (OtherActor :type Actor%20Object%20Reference))
  (|CallParentFunction OtherActor) ; This node is disabled and will not be called.\nDrag off pins to build functionality.
)

(event EventTick
  (params (DeltaSeconds :type Float%20%28single-precision%29))
  (|CallParentFunction DeltaSeconds) ; This node is disabled and will not be called.\nDrag off pins to build functionality.
)

(fn ConstructionScript
  (|CallParentFunction))