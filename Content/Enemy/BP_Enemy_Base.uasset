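; Base enemy pawn that works with AIC_Enemy_Base and sets it to passive shortly after spawning.
; Chase moves toward the player controller, then on success triggers Attack, which deals heavy damage to the player character without a range check.
; Attack and Chase call end notifications, while helper functions expose attack and strafe radii, a patrol path, and enum-based movement speed presets.
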(event Custom|Attack
  (bind _returnvalue (Game|Damage|ApplyDamage (Game|GetPlayerCharacter 0) 1e+02 0 self "/Script/Engine.DamageType"))
  (Development|PrintString (Utilities|String|ToString(Float) _returnvalue) true false "(R=1.000000,G=0.000000,B=0.075629,A=1.000000)" 1.0)
  (Default|CallOnAttackEnd))

(event Custom|Chase
  (AI|AIMoveTo self "0, 0, 0" (Game|GetPlayerController 0) 2e+01 true
    (:OnSuccess
      (CallFunction|Attack)
      (Default|CallOnChaseEnd))))

(event EventBeginPlay
  (Utilities|FlowControl|Delay 0.2)
  (bind _asaic_enemy_base (Utilities|Casting|CastToAIC_Enemy_Base (AI|GetAIController 0)))
  (Default|SetStatePassive _asaic_enemy_base))

(fn ConstructionScript)

(fn GetIdealRange
  (return 4e+01 3.5e+02))

(fn GetPatrolPath
  (return (Variables|Default|GetPatrol%20Path)))

(fn SetMovementSpeed
  (params (Speeds :type E_Speeds%20Enum :default "NewEnumerator0"))
  (bind _output_get (Variables|/Script/Engine.CharacterMovementComponent|SetMaxWalkSpeed (Variables|Character|GetCharacterMovement) (Utilities|Select :Index Speeds :NewEnumerator0 0.0 :NewEnumerator1 3.5e+02 :NewEnumerator2 525.0 :NewEnumerator3 7e+02)))
  (bind _output_get_2 (Variables|Default|SetRun%20Speed _output_get))
  (return _output_get_2))