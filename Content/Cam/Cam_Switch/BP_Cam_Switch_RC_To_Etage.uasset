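; Camera switch trigger that changes the third-person character's spring arm between ground-floor (RC) and upper-floor (Etage, 1st/2nd) framing.
; Entering the Box applies the RC location and arm length, a chain also wired to BeginPlay through the overlap's OtherActor.
; Leaving the Box applies the Etage location, rotation and arm length.
; Both changes are instant, with no blending.
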(event OnComponentBeginOverlap(Box)
  (params (OverlappedComponent :type Primitive%20Component%20Object%20Reference) (OtherActor :type Actor%20Object%20Reference) (OtherComp :type Primitive%20Component%20Object%20Reference) (OtherBodyIndex :type Integer) (bFromSweep :type Boolean) (SweepResult :type Hit%20Result%20Structure%20%28by%20ref%29))
  ;[1 1 1] RC
  (bind _asbp_third_person_character (Utilities|Casting|CastToBP_ThirdPersonCharacter OtherActor))
  (Transformation|SetRelativeTransform (Variables|/Game/ThirdPerson/Blueprints/BP_ThirdPersonCharacter.BP_ThirdPersonCharacter_C|GetSpringArm _asbp_third_person_character) (Math|Transform|MakeTransform (Variables|Default|GetRC%20/%20Location%20Cam) "0, 0, 0" "1.000000,1.000000,1.000000") false false)
  (Variables|/Script/Engine.SpringArmComponent|SetTargetArmLength (Variables|/Game/ThirdPerson/Blueprints/BP_ThirdPersonCharacter.BP_ThirdPersonCharacter_C|GetSpringArm _asbp_third_person_character) (Variables|Default|GetRC%20/%20Distance%20Cam)))

(event OnComponentEndOverlap(Box)
  (params (OverlappedComponent :type Primitive%20Component%20Object%20Reference) (OtherActor :type Actor%20Object%20Reference) (OtherComp :type Primitive%20Component%20Object%20Reference) (OtherBodyIndex :type Integer))
  ;[1 1 1] 1er / 2eme
  (bind _asbp_third_person_character (Utilities|Casting|CastToBP_ThirdPersonCharacter OtherActor))
  (Transformation|SetRelativeTransform (Variables|/Game/ThirdPerson/Blueprints/BP_ThirdPersonCharacter.BP_ThirdPersonCharacter_C|GetSpringArm _asbp_third_person_character) (Math|Transform|MakeTransform (Variables|Default|GetEtage%20/%20Location%20Cam) (Variables|Default|GetEtage%20/%20Rota%20Cam) "1.000000,1.000000,1.000000") false false)
  (Variables|/Script/Engine.SpringArmComponent|SetTargetArmLength (Variables|/Game/ThirdPerson/Blueprints/BP_ThirdPersonCharacter.BP_ThirdPersonCharacter_C|GetSpringArm _asbp_third_person_character) (Variables|Default|GetEtage%20/%20Distance%20Cam)))

(event EventBeginPlay
  ;[1 1 1] RC
  (bind _asbp_third_person_character (Utilities|Casting|CastToBP_ThirdPersonCharacter (stale OnComponentBeginOverlap(Box) OtherActor)))
  (Transformation|SetRelativeTransform (Variables|/Game/ThirdPerson/Blueprints/BP_ThirdPersonCharacter.BP_ThirdPersonCharacter_C|GetSpringArm _asbp_third_person_character) (Math|Transform|MakeTransform (Variables|Default|GetRC%20/%20Location%20Cam) "0, 0, 0" "1.000000,1.000000,1.000000") false false)
  (Variables|/Script/Engine.SpringArmComponent|SetTargetArmLength (Variables|/Game/ThirdPerson/Blueprints/BP_ThirdPersonCharacter.BP_ThirdPersonCharacter_C|GetSpringArm _asbp_third_person_character) (Variables|Default|GetRC%20/%20Distance%20Cam)))

(fn ConstructionScript)