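; Intro camera actor for the tutorial level that runs a timed opening sequence on BeginPlay.
; It disables player input, freezes BP_Timer and plays a WBP_Transi_Level_Tuto fade-in and fade-out transition.
; As the fade-out starts, the view cuts to this actor, holds, then blends cubically back to the player character.
; Once the blend ends, the timer unfreezes and input returns, with all steps sequenced by fixed delays.
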(event EventBeginPlay
  (bind _returnvalue (Game|GetPlayerController 0))
  (bind _returnvalue_2 (Game|GetPlayerCharacter 0))
  (Input|DisableInput (Game|GetPlayerCharacter 0) (Game|GetPlayerController 0))
  (Utilities|FlowControl|Delay 0.2)
  (bind _returnvalue_3 (Actor|GetActorOfClass "/Game/Widgets/Timer/BP_Timer.BP_Timer_C"))
  (Default|FFreeze _returnvalue_3)
  (bind _returnvalue_4 (UserInterface|CreateWidget "/Game/Widgets/Transi_Level/WBP_Transi_Level_Tuto.WBP_Transi_Level_Tuto_C"))
  (UserInterface|Viewport|AddtoViewport _returnvalue_4 0)
  (Default|FadeinTransi _returnvalue_4)
  (Utilities|FlowControl|Delay 2.85)
  (Default|FadeOutTransi _returnvalue_4)
  (Game|Player|SetViewTargetwithBlend _returnvalue self 0.0 "VTBlend_PreBlended" 0.0 false)
  (Utilities|FlowControl|Delay 5.5)
  (Game|Player|SetViewTargetwithBlend _returnvalue _returnvalue_2 3.0 "VTBlend_Cubic" 0.0 false)
  (Utilities|FlowControl|Delay 3.0)
  (Default|FUnfreeze _returnvalue_3)
  (Input|EnableInput _returnvalue_2 _returnvalue))

(fn ConstructionScript)