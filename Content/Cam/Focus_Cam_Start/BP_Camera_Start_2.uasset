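; Camera actor that plays the Level 2 intro cinematic when the level begins.
; On BeginPlay it disables player input, freezes BP_Timer and runs a fade transition widget.
; It then makes itself the view target and plays the Level_2 sequence.
; After timed delays it blends back to the player character, unfreezes the timer and restores input.
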(event EventBeginPlay
  (bind _returnvalue (Game|GetPlayerCharacter 0))
  (bind _returnvalue_2 (Game|GetPlayerCharacter 0))
  (bind _returnvalue_3 (Game|GetPlayerController 0))
  (bind _outactor (Sequencer|Player|CreateLevelSequencePlayer "/Game/tests/Level_2.Level_2"))
  (Input|DisableInput _returnvalue (Game|GetPlayerController 0))
  (bind _returnvalue_4 (UserInterface|CreateWidget "/Game/Widgets/Transi_Level/WBP_Transi_Level_2.WBP_Transi_Level_2_C"))
  (UserInterface|Viewport|AddtoViewport _returnvalue_4 0)
  (Utilities|FlowControl|Delay 0.2)
  (bind _returnvalue_5 (Actor|GetActorOfClass "/Game/Widgets/Timer/BP_Timer.BP_Timer_C"))
  (Default|FFreeze _returnvalue_5)
  (Default|FadeinTransi _returnvalue_4)
  (Utilities|FlowControl|Delay 2.85)
  (Default|FadeOutTransi _returnvalue_4)
  (Input|DisableInput _returnvalue_2 _returnvalue_3)
  (Game|Player|SetViewTargetwithBlend _returnvalue_3 self 0.0 "VTBlend_PreBlended" 0.0 false)
  (Sequencer|Player|Play (Variables|/Script/LevelSequence.LevelSequenceActor|GetSequencePlayer _outactor) :!class /Script/MovieScene.MovieSceneSequencePlayer)
  (Utilities|FlowControl|Delay 5.65)
  (Game|Player|SetViewTargetwithBlend _returnvalue_3 _returnvalue_2 3.0 "VTBlend_Cubic" 0.0 false)
  (Utilities|FlowControl|Delay 3.0)
  (Default|FUnfreeze (Variables|/Game/ThirdPerson/Blueprints/BP_ThirdPersonCharacter.BP_ThirdPersonCharacter_C|GetVTimer (.AsBP%20Third%20Person%20Character (Utilities|Casting|CastToBP_ThirdPersonCharacter _returnvalue))))
  (Input|EnableInput _returnvalue_2 _returnvalue_3))

(fn ConstructionScript)